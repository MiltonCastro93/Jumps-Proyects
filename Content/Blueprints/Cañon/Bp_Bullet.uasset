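; Cannon bullet projectile that damages the player on contact.
; The construction script sets the projectile movement's forward velocity and max speed from Speed.
; On sphere overlap, the VerificacionCharacter macro filters for the player, then Damage is applied scaled by the selected difficulty index from GI_Instancias.
; The bullet destroys itself after applying damage, and this graph does nothing on other overlaps.
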(event `self.Sphere.OnComponentBeginOverlap`
  (params (OverlappedComponent :type "PrimitiveComponent Object Reference") (OtherActor :type "Actor Object Reference") (OtherComp :type "PrimitiveComponent Object Reference") (OtherBodyIndex :type Integer) (bFromSweep :type Boolean) (SweepResult :type "HitResult Structure (by ref)"))
  ;[0 0 0 0.5] Daño al Jugador
  (`/Game/Blueprints/Librerias/ML_BP_Verificacion.VerificacionCharacter` OtherActor
    (:`Is Player`
      (bind _asgi_instancias (cast `/Game/Blueprints/Core/GI_Instancias` (`GameplayStatics.GetGameInstance`)))
      (bind (_dificultad_seleccionada_id _dificultad_seleccionada_nombreamostrar _dificultad_seleccionada_indice) (break `/Game/Blueprints/Datas/S_Dificultad` (`/Game/Blueprints/Core/GI_Instancias.Dificultad Seleccionada` _asgi_instancias)))
      (`GameplayStatics.ApplyDamage` OtherActor (* (`self.Damage`) _dificultad_seleccionada_indice) null self)
      (`self.K2_DestroyActor`))))

(fn `UserConstructionScript`
  (bind _projectilemovement (`self.ProjectileMovement`))
  (set `MovementComponent.Velocity` (`KismetMathLibrary.MakeVector` (`self.Speed`)) _projectilemovement)
  (set `ProjectileMovementComponent.MaxSpeed` (`self.Speed`) _projectilemovement))