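; Rotating platform actor with four floor pieces that spins only while the player character is inside its Box trigger.
; Entering the trigger activates a RotatingMovement component, and Tick resets each floor's world rotation to zero so the floors stay level, Ferris-wheel style.
; Leaving deactivates the movement, which snaps the actor to a fixed rotation, re-levels the floors and prints a debug message.
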(event `self.RotatingMovement.OnComponentActivated`
  (params (Component :type "ActorComponent Object Reference") (bReset :type Boolean))
  ;[0 0 0 0.5] (De)/Activated RotationMovement
  (`KismetSystemLibrary.PrintString` "Activado"))

(event `self.RotatingMovement.OnComponentDeactivated`
  (params (Component :type "ActorComponent Object Reference"))
  ;[0 0 0 0.5] (De)/Activated RotationMovement
  (`KismetSystemLibrary.PrintString` "DesActivado")
  (`self.K2_SetActorRotation` (struct :`Yaw` 90.0))
  (`self.Turn`))

(event `self.ReceiveTick`
  (params (DeltaSeconds :type "Float (single-precision)"))
  ;[0 0 0 0.5] Event Tick
  (if (`self.TurnPlataforms`)
    (`self.Turn`)))

(event `Turn`
  ;[0 0 0 0.5] Rota las Plataformas
  (`SceneComponent.K2_SetWorldRotation` :`self` (`self.Piso1`))
  (`SceneComponent.K2_SetWorldRotation` :`self` (`self.Piso2`))
  (`SceneComponent.K2_SetWorldRotation` :`self` (`self.Piso3`))
  (`SceneComponent.K2_SetWorldRotation` :`self` (`self.Piso4`)))

(event `self.Box.OnComponentBeginOverlap`
  (params (OverlappedComponent :type "PrimitiveComponent Object Reference") (OtherActor :type "Actor Object Reference") (OtherComp :type "PrimitiveComponent Object Reference") (OtherBodyIndex :type Integer) (bFromSweep :type Boolean) (SweepResult :type "HitResult Structure (by ref)"))
  ;[0 0 0 0.5] Starts/End Overlaps
  (if (== OtherActor (`GameplayStatics.GetPlayerCharacter` 0))
    (`ActorComponent.Activate` (`self.RotatingMovement`) false)
    (set `self.TurnPlataforms` true)))

(event `self.Box.OnComponentEndOverlap`
  (params (OverlappedComponent :type "PrimitiveComponent Object Reference") (OtherActor :type "Actor Object Reference") (OtherComp :type "PrimitiveComponent Object Reference") (OtherBodyIndex :type Integer))
  ;[0 0 0 0.5] Starts/End Overlaps
  (if (== OtherActor (`GameplayStatics.GetPlayerCharacter` 0))
    (`ActorComponent.Deactivate` (`self.RotatingMovement`))
    (set `self.TurnPlataforms` false)))

(fn `UserConstructionScript`)