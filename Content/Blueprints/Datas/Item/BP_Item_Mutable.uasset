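; BP_Item_Mutable is a data-driven pickup that acts as either a tomato or a health potion.
; The construction script reads its DT_Items row to set the static mesh and item type.
; On sphere overlap, a library macro confirms the player, then a tomato calls TestCurrent on GM_Saltarin, while a potion changes health through GI_Instancias.
; The item destroys itself once that effect is applied.
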(event `self.Sphere.OnComponentBeginOverlap`
  (params (OverlappedComponent :type "PrimitiveComponent Object Reference") (OtherActor :type "Actor Object Reference") (OtherComp :type "PrimitiveComponent Object Reference") (OtherBodyIndex :type Integer) (bFromSweep :type Boolean) (SweepResult :type "HitResult Structure (by ref)"))
  (switch `/Game/Blueprints/Datas/E_TipoItem` (`self.Tipo`)
    (:`NewEnumerator0`
      ;[0 0 0 0.5] Tomate
      ;;[0 0 0 0.5] Macro Libreria
      (`/Game/Blueprints/Librerias/ML_BP_Verificacion.VerificacionCharacter` OtherActor
        (:`Is Player`
          (bind _asgm_saltarin (cast `/Game/Blueprints/Core/GM_Saltarin` (`GameplayStatics.GetGameMode`)))
          (`/Game/Blueprints/Core/GM_Saltarin.TestCurrent` _asgm_saltarin)
          (`self.K2_DestroyActor`))))
    (:`NewEnumerator1`
      ;[0 0 0 0.5] Pocima
      (`/Game/Blueprints/Librerias/ML_BP_Verificacion.VerificacionCharacter` OtherActor
        (:`Is Player`
          (bind _asgi_instancias (cast `/Game/Blueprints/Core/GI_Instancias` (`GameplayStatics.GetGameInstance`)))
          (`/Game/Blueprints/Core/GI_Instancias.Modificar Vida` _asgi_instancias 50.0)
          (`self.K2_DestroyActor`))))))

(fn `UserConstructionScript`
  (bind (_item_data_datatable _item_data_rowname) (break `DataTableRowHandle` (`self.Item Data`)))
  (bind _returnvalue (`|GetDataTableRow` "/Game/Blueprints/Datas/DT_Items.DT_Items" _item_data_rowname)
    (:`then`
      (bind (_id _nombreamostrar _descripcion _drop _icono _staticmesh _tipo) (break `/Game/Blueprints/Datas/S_Item` _returnvalue))
      (`StaticMeshComponent.SetStaticMesh` (`self.StaticMesh`) _staticmesh)
      (set `self.Tipo` _tipo))
    (:`RowNotFound`
      (`KismetSystemLibrary.PrintString` "Error" true true (struct :`R` 1.0 :`A` 1.0)))))