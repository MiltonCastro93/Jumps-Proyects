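; GM_Saltarin is the game mode that tracks collected tomatoes and decides victory.
; TestCurrent increments the tomato count and passes it with the maximum to PC_Saltarin through EnviarInfoAlHUD for the HUD.
; VerificaciondeVictoria compares the count to the maximum, then either prints a win message and opens L_Nivel01 after a delay, or prints collected and remaining tomatoes.
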(event `TestCurrent`
  ;[0 0 0 0.5] Suma de Tomates
  (bind _result (`/Engine/EditorBlueprintResources/StandardMacros.IncrementInt` (`self.CurrentTomate`))
    (:`  `
      (set `self.CurrentTomate` _result)
      ;[0 0 0 0.5] Comunicacion del GameMode -> PlayerController
      (bind _aspc_saltarin (cast `/Game/Blueprints/Core/PC_Saltarin` (`GameplayStatics.GetPlayerController` 0)))
      (`/Game/Blueprints/Core/PC_Saltarin.Enviar Info al HUD` _aspc_saltarin (`self.CurrentTomate`) (`self.TomateMax`)))))

(event `Verificacion de Victoria`
  ;[0 0 0 0.5] Verificar el estado de Victoria
  (if (>= (`self.CurrentTomate`) (`self.TomateMax`))
    (`KismetSystemLibrary.PrintString` "Ganaste")
    (`KismetSystemLibrary.Delay` 5.0)
    (`GameplayStatics.OpenLevelBySoftObjectPtr` "/Game/Level/L_Nivel01.L_Nivel01")
    (else
      (`KismetSystemLibrary.PrintString` (`KismetStringLibrary.Concat_StrStr` "Tenes: " (`KismetStringLibrary.Conv_IntToString` (`self.CurrentTomate`)) " / Te faltan: " (`KismetStringLibrary.Conv_IntToString` (- (`self.TomateMax`) (`self.CurrentTomate`)))) true true (struct :`G` 0.996309 :`B` 1.0 :`A` 1.0)))))

(fn `UserConstructionScript`)