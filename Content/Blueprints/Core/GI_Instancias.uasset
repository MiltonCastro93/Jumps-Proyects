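; GI_Instancias is the Game Instance that holds the selected difficulty and the player's health.
; On Init it loads the "Facil" row from DT_Dificultades as default; a menu selection replaces it and starts the match through PC_Saltarin.
; Health changes are capped at the maximum and sent to the HUD through PC_Saltarin.
; At zero health it flags death, opens L_Nivel01 and refills health.
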(event `SeleccionMODE`
  (params (ModoSeleccionado :type "/Game/Blueprints/Datas/S_Dificultad Structure"))
  ;[0 0 0 0.5] Comunicacion entre WBP_Menu -> Self -> PlayerController
  (set `self.Dificultad Seleccionada` ModoSeleccionado)
  (bind _aspc_saltarin (cast `/Game/Blueprints/Core/PC_Saltarin` (`GameplayStatics.GetPlayerController` 0)))
  (`/Game/Blueprints/Core/PC_Saltarin.Iniciar Partida` _aspc_saltarin))

(event `self.ReceiveInit`
  ;[0 0 0 0.5] Un tipo Start o begin Play
  (bind _returnvalue (`|GetDataTableRow` "/Game/Blueprints/Datas/DT_Dificultades.DT_Dificultades" "Facil")
    (:`then`
      (set `self.Dificultad Seleccionada` _returnvalue))))

(event `Modificar Vida`
  (params (Value :type "Float (double-precision)"))
  ;[0 0 0 0.5] Evaluamos si supero la vida max
  (bind _output_get (set `self.VidaCurrent` (+ (`self.VidaCurrent`) Value)))
  (if (> _output_get (`self.VidaMax`))
    (set `self.VidaCurrent` (`self.VidaMax`)))
  ;[0 0 0 0.5] Actualizar la Vida. (Self -> PlayerController)
  (bind _aspc_saltarin (cast `/Game/Blueprints/Core/PC_Saltarin` (`GameplayStatics.GetPlayerController` 0)))
  (`/Game/Blueprints/Core/PC_Saltarin.Enviar Info Vida al HUD` _aspc_saltarin (`self.VidaCurrent`))
  ;[0 0 0 0.5] Evalua si estamos muertos
  (if (<= (`self.VidaCurrent`) 0.0)
    (set `self.IsDead?` true)
    (`GameplayStatics.OpenLevelBySoftObjectPtr` "/Game/Level/L_Nivel01.L_Nivel01")
    (set `self.VidaCurrent` (`self.VidaMax`))
    (else
      (set `self.IsDead?` false))))