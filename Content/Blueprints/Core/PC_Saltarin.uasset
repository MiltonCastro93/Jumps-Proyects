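; Player controller that manages the main menu and in-game HUD, relaying game state to the UI.
; On BeginPlay it stops the third-person character and shows WBP_Menu with the cursor visible.
; IniciarPartida removes the menu, creates WBP_Hud and releases the character.
; Events forward item counts and life to the HUD, lazily creating it through a guarded function that stores its reference.
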(event `self.ReceiveBeginPlay`
  (bind _returnvalue (`GameplayStatics.GetPlayerCharacter` 0))
  ;[0 0 0 0.5] Instancio primero el HUD del Menu
  (`/Engine/EditorBlueprintResources/StandardMacros.IsValid` _returnvalue
    (:`Is Valid`
      (bind _asbp_third_person_character (cast `/Game/ThirdPerson/Blueprints/BP_ThirdPersonCharacter` _returnvalue))
      (`/Game/ThirdPerson/Blueprints/BP_ThirdPersonCharacter.StopMovement` _asbp_third_person_character)
      (`self.HUD MENU`))))

(event `Iniciar Partida`
  (bind _returnvalue (`GameplayStatics.GetPlayerCharacter` 0))
  ;[0 0 0 0.5] Comunicacion entre UI HUD (WBP_Menu) -> GameInstance -> Self para activar el HUD del juego
  (`Widget.RemoveFromParent` (`self.HUD MenuREF`))
  (`self.CREAR HUD`)
  (`/Engine/EditorBlueprintResources/StandardMacros.IsValid` _returnvalue
    (:`Is Valid`
      (bind _asbp_third_person_character (cast `/Game/ThirdPerson/Blueprints/BP_ThirdPersonCharacter` _returnvalue))
      (`/Game/ThirdPerson/Blueprints/BP_ThirdPersonCharacter.PlayPlayer` _asbp_third_person_character))))

(event `Enviar Info al HUD`
  (params (Value :type Integer) (MaxItems :type Integer))
  ;[0 0 0 0.5] Comunicacion entre GameMode -> Self -> UI HUD
  (bind _hud_ref (`self.Hud REF`)
    (:`then`
      _)
    (:`else`
      (`KismetSystemLibrary.PrintString` "No esta Creado el HUD" true true (struct :`R` 1.0 :`A` 1.0))
      (`self.CREAR HUD`)
      (`KismetSystemLibrary.PrintString` "Ya Instanciado el HUD" true true (struct :`G` 1.0 :`A` 1.0))))
  (`/Game/UI/HUD/WBP_Hud.Modificar Valor HUD` _hud_ref Value MaxItems))

(event `Enviar Info Vida al HUD`
  (params (Life :type "Float (double-precision)"))
  ;[0 0 0 0.5] Comunicacion entre GameInstance -> Self -> UI HUD
  (bind _hud_ref (`self.Hud REF`)
    (:`then`
      _)
    (:`else`
      (`self.CREAR HUD`)))
  (`/Game/UI/HUD/WBP_Hud.Modificar Vida` _hud_ref Life))

(fn `CREAR HUD`
  (`self.Hud REF`
    (:`then`)
    (:`else`
      ;[0 0 0 0.5] Creo el HUD WIDGET, Almaceno su Ref
      (bind _returnvalue (`|CreateWidget` "/Game/UI/HUD/WBP_Hud.WBP_Hud_C"))
      (bind _output_get (set `self.Hud REF` _returnvalue))
      ;[0 0 0 0.5] Lo agrego al ViewPort
      (`UserWidget.AddToViewport` _output_get 0)
      ;[1 0 0 0.5] Metodo de Interaccion
      (`WidgetBlueprintLibrary.SetInputMode_GameOnly` self)
      (set `self.bShowMouseCursor` false))))

(fn `HUD MENU`
  (`self.HUD MenuREF`
    (:`then`)
    (:`else`
      (bind _returnvalue (`|CreateWidget` "/Game/UI/HUD/WBP_Menu.WBP_Menu_C"))
      (bind _output_get (set `self.HUD MenuREF` _returnvalue))
      (`UserWidget.AddToViewport` _output_get 0)
      (`WidgetBlueprintLibrary.SetInputMode_GameOnly` self)
      (set `self.bShowMouseCursor` true))))

(fn `UserConstructionScript`)