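; Tomato pickup actor that the player collects by overlapping its sphere in the Saltarin game mode.
; An overlap that the VerificacionCharacter library macro confirms as the player activates a Niagara effect and plays the pickup sound.
; The Niagara component's activation event then waits briefly, calls TestCurrent on GM_Saltarin to report the collection, and destroys the actor.
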(event `self.ReceiveBeginPlay`
  (`AudioComponent.Stop` (`self.Pick_Up_Item`)))

(event `self.Sphere.OnComponentBeginOverlap`
  (params (OverlappedComponent :type "PrimitiveComponent Object Reference") (OtherActor :type "Actor Object Reference") (OtherComp :type "PrimitiveComponent Object Reference") (OtherBodyIndex :type Integer) (bFromSweep :type Boolean) (SweepResult :type "HitResult Structure (by ref)"))
  ;[0 0 0 0.5] Macro Libreria
  (`/Game/Blueprints/Librerias/ML_BP_Verificacion.VerificacionCharacter` OtherActor
    (:`Is Player`
      (`ActorComponent.Activate` (`self.NewNiagaraSystem`) false)
      (`AudioComponent.Play` (`self.Pick_Up_Item`) 0.0))))

(event `self.NewNiagaraSystem.OnComponentActivated`
  (params (Component :type "ActorComponent Object Reference") (bReset :type Boolean))
  ;[0 0 0 0.5] Comunicacion entre Self -> GameMode (Info sobre la Obtencion del item)
  ;;[0 0 0 0.5] Cuando se activa, espera 4s, y hace su magia!
  (`KismetSystemLibrary.Delay` 0.7)
  (bind _asgm_saltarin (cast `/Game/Blueprints/Core/GM_Saltarin` (`GameplayStatics.GetGameMode`)))
  (`/Game/Blueprints/Core/GM_Saltarin.TestCurrent` _asgm_saltarin)
  (`self.K2_DestroyActor`))

(fn `UserConstructionScript`)