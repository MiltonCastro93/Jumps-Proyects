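; Box item Blueprint that displays an integer value and can be moved back to a given position.
; On BeginPlay it writes Value into the Count text.
; The Reposition event sets the static mesh's world location directly, without sweep, leaving rotation untouched.
; The mesh hit event does nothing, and a debug check for box tilt on player contact is left disconnected.
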(event `self.ReceiveBeginPlay`
  (`TextRenderComponent.K2_SetText` (`self.Count`) (`KismetTextLibrary.Conv_IntToText` (`self.Value`))))

(event `self.StaticMesh.OnComponentHit`
  (params (HitComponent :type "PrimitiveComponent Object Reference") (OtherActor :type "Actor Object Reference") (OtherComp :type "PrimitiveComponent Object Reference") (NormalImpulse :type "Vector Structure") (Hit :type "HitResult Structure (by ref)")))

(event `Reposition`
  (params (Position :type "Vector Structure"))
  ;[0 0 0 0.5] Reestablecer Posicion de la Caja
  (`SceneComponent.K2_SetWorldLocation` (`self.StaticMesh`) Position false false))

(fn `UserConstructionScript`)