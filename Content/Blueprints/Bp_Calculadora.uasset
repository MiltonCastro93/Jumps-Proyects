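; Bp_Calculadora is a practice calculator Blueprint, apparently demonstrating local macros and functions for modular code.
; On BeginPlay it runs the Calculadora macro, then prints "Hola Mundo".
; The macro waits briefly, passes two values through separate add, subtract, multiply and divide helpers, and prints the labeled results as one colored on-screen string.
; Other helper calls in the event graph are disconnected examples that never run.
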(event `self.ReceiveBeginPlay`
  ; MacroLocal
  (`self.Calculadora`)
  (`KismetSystemLibrary.PrintString` "Hola Mundo"))

(fn `Restar 2 Valores`
  (params (ValueA :type "Float (double-precision)") (ValueB :type "Float (double-precision)"))
  (returns (Resultado :type "Float (double-precision)"))
  (return (- ValueA ValueB)))

(fn `Sumar 2 Valores`
  (params (ValueA :type "Float (double-precision)") (ValueB :type "Float (double-precision)"))
  (returns (Resultado :type "Float (double-precision)"))
  (return (+ ValueA ValueB)))

(fn `UserConstructionScript`)