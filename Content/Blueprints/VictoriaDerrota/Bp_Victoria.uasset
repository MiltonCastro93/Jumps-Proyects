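; Victory trigger actor that marks where the player triggers the win check.
; On BeginPlay it stops its GameComplete audio so it stays silent until triggered.
; When the player character overlaps its Box, it calls VerificacionDeVictoria on GM_Saltarin, which owns the victory logic, then plays GameComplete without waiting for the result.
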(event `self.ReceiveBeginPlay`
  (`AudioComponent.Stop` (`self.Game_Complete`)))

(event `self.Box.OnComponentBeginOverlap`
  (params (OverlappedComponent :type "PrimitiveComponent Object Reference") (OtherActor :type "Actor Object Reference") (OtherComp :type "PrimitiveComponent Object Reference") (OtherBodyIndex :type Integer) (bFromSweep :type Boolean) (SweepResult :type "HitResult Structure (by ref)"))
  (if (== OtherActor (`GameplayStatics.GetPlayerCharacter` 0))
    (bind _asgm_saltarin (cast `/Game/Blueprints/Core/GM_Saltarin` (`GameplayStatics.GetGameMode`)))
    (`/Game/Blueprints/Core/GM_Saltarin.Verificacion de Victoria` _asgm_saltarin)
    (`AudioComponent.Play` (`self.Game_Complete`) 0.0)))

(fn `UserConstructionScript`)