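; Automatic door Blueprint that swings open when the player enters its trigger box and closes when they leave.
; Box overlap events filter for the player through VerificacionCharacter, then play or reverse the MovimientoDeLaPuerta timeline.
; The timeline's rotation curve drives the door's relative yaw via SetearRotacion, keeping roll and pitch, with an Invertido flag flipping the swing direction.
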(event `self.Box.OnComponentBeginOverlap`
  (params (OverlappedComponent :type "PrimitiveComponent Object Reference") (OtherActor :type "Actor Object Reference") (OtherComp :type "PrimitiveComponent Object Reference") (OtherBodyIndex :type Integer) (bFromSweep :type Boolean) (SweepResult :type "HitResult Structure (by ref)"))
  ;[0 0 0 0.5] Identificacion del Player
  (`/Game/Blueprints/Librerias/ML_BP_Verificacion.VerificacionCharacter` OtherActor
    (:`Is Player`
      ;[0 0 0 0.5] Apertura de la puerta
      (bind (_direction _rotacionpuerta) (`Timeline|Movimiento de la Puerta` :!label _label)
        (:`Update`
          (if (`self.Invertido?`)
            (`self.Setear Rotacion` (* _rotacionpuerta -1.0))
            (else
              (`self.Setear Rotacion` _rotacionpuerta))))
        (:`Finished`
          (`KismetSystemLibrary.PrintString` "Finalizo"))))))

(event `self.Box.OnComponentEndOverlap`
  (params (OverlappedComponent :type "PrimitiveComponent Object Reference") (OtherActor :type "Actor Object Reference") (OtherComp :type "PrimitiveComponent Object Reference") (OtherBodyIndex :type Integer))
  (`/Game/Blueprints/Librerias/ML_BP_Verificacion.VerificacionCharacter` OtherActor
    (:`Is Player`
      (goto _label :!via `Reverse`))))

(fn `UserConstructionScript`)