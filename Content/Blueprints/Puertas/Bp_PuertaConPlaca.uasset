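; Door Blueprint that swings open and closed through the AbrirPuerta and CerrarPuerta events, named for use with a plate, though no trigger logic lives here.
; The MovimientoDeLaPuerta timeline drives the relative yaw of Puerta, with Invertido flipping the swing direction.
; Closing reverses the same timeline.
; OpenDoor is silenced on BeginPlay, plays when opening starts and stops when the timeline finishes.
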(event `self.ReceiveBeginPlay`
  (`AudioComponent.Stop` (`self.OpenDoor`)))

(event `Abrir Puerta`
  (bind _puerta (`self.Puerta`))
  (bind _puerta_2 (`self.Puerta`))
  (bind (_relativerotation_roll _relativerotation_pitch) (`KismetMathLibrary.BreakRotator` (`SceneComponent.RelativeRotation` _puerta)))
  (bind (_relativerotation_roll_2 _relativerotation_pitch_2) (`KismetMathLibrary.BreakRotator` (`SceneComponent.RelativeRotation` _puerta_2)))
  ;[0 0 0 0.5] Apertura de la puerta
  (`AudioComponent.Play` (`self.OpenDoor`) 0.0)
  (bind (_direction _rotacionpuerta) (`Timeline|Movimiento de la Puerta` :!label _label)
    (:`Update`
      (if (`self.Invertido?`)
        (`SceneComponent.K2_SetRelativeRotation` _puerta (`KismetMathLibrary.MakeRotator` _relativerotation_roll _relativerotation_pitch (* _rotacionpuerta -1.0)) false false)
        (else
          (`SceneComponent.K2_SetRelativeRotation` _puerta_2 (`KismetMathLibrary.MakeRotator` _relativerotation_roll_2 _relativerotation_pitch_2 _rotacionpuerta) false false))))
    (:`Finished`
      (`AudioComponent.Stop` (`self.OpenDoor`)))))

(event `Cerrar Puerta`
  ;[0 0 0 0.5] Apertura de la puerta
  (goto _label :!via `Reverse`))

(fn `UserConstructionScript`)