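; Pressure plate actor that opens a linked Bp_PuertaConPlaca door while the player or a referenced barrel stands on it.
; Box overlaps set the pressed flag and play or reverse a timeline that moves the button within a clamped Z range.
; When the timeline finishes, the plate synchronously loads the door from a soft reference, casts it and opens or closes it by that flag, with debug prints.
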(event `self.Box.OnComponentBeginOverlap`
  (params (OverlappedComponent :type "PrimitiveComponent Object Reference") (OtherActor :type "Actor Object Reference") (OtherComp :type "PrimitiveComponent Object Reference") (OtherBodyIndex :type Integer) (bFromSweep :type Boolean) (SweepResult :type "HitResult Structure (by ref)"))
  (bind _boton (`self.Boton`))
  (bind _boton_2 (`self.Boton`))
  (bind (_relativelocation_x _relativelocation_y _relativelocation_z) (`KismetMathLibrary.BreakVector` (`SceneComponent.RelativeLocation` _boton)))
  (bind (_relativelocation_x_2 _relativelocation_y_2 _relativelocation_z_2) (`KismetMathLibrary.BreakVector` (`SceneComponent.RelativeLocation` _boton_2)))
  ;[0 0 0 0.5] Comparacion del Player/Determinado Go sobre la placa
  (if (or (== OtherActor (`GameplayStatics.GetPlayerCharacter` 0)) (== OtherActor (`self.Barril REF`)))
    (set `self.Presionando` true)
    (bind (_direction _position) (`Timeline|Activar Placa` :!label _label)
      (:`Update`
        (if (`self.Presionando`)
          ;[0 0 0 0.5] Baja la Placa de Presion
          (`SceneComponent.K2_SetRelativeLocation` _boton_2 (`KismetMathLibrary.MakeVector` _relativelocation_x_2 _relativelocation_y_2 (`KismetMathLibrary.FClamp` (- _relativelocation_z_2 _position) 6.0 11.0)) true false)
          (else
            ;[0 0 0 0.5] Sube la Placa de Presion
            (`SceneComponent.K2_SetRelativeLocation` _boton (`KismetMathLibrary.MakeVector` _relativelocation_x _relativelocation_y (`KismetMathLibrary.FClamp` (+ _relativelocation_z _position) 6.0 11.0)) true false))))
      (:`Finished`
        (if (`self.Presionando`)
          ;[0 0 0 0.5] Para Abrir La Puerta
          ;; Error Controlado ref!=null
          (bind _puerta_ref (`self.Puerta REF`)
            (:`then`
              (bind _returnvalue (`KismetSystemLibrary.LoadAsset_Blocking` _puerta_ref))
              (bind _asbp_puerta_con_placa (cast `/Game/Blueprints/Puertas/Bp_PuertaConPlaca` _returnvalue))
              (`/Game/Blueprints/Puertas/Bp_PuertaConPlaca.Abrir Puerta` _asbp_puerta_con_placa)
              (`KismetSystemLibrary.PrintString` "Puerta Activada"))
            (:`else`
              (`KismetSystemLibrary.PrintString` "La puerta no esta Asignada")))
          (else
            ;[0 0 0 0.5] Para Cerrar la Puerta
            (bind _puerta_ref_2 (`self.Puerta REF`)
              (:`then`
                (bind _returnvalue_2 (`KismetSystemLibrary.LoadAsset_Blocking` _puerta_ref_2))
                (bind _asbp_puerta_con_placa_2 (cast `/Game/Blueprints/Puertas/Bp_PuertaConPlaca` _returnvalue_2))
                (`/Game/Blueprints/Puertas/Bp_PuertaConPlaca.Cerrar Puerta` _asbp_puerta_con_placa_2)
                (`KismetSystemLibrary.PrintString` "La Puerta se Estara Cerrando."))
              (:`else`
                (`KismetSystemLibrary.PrintString` "La puerta no esta Asignada")))))))))

(event `self.Box.OnComponentEndOverlap`
  (params (OverlappedComponent :type "PrimitiveComponent Object Reference") (OtherActor :type "Actor Object Reference") (OtherComp :type "PrimitiveComponent Object Reference") (OtherBodyIndex :type Integer))
  (if (or (== OtherActor (`GameplayStatics.GetPlayerCharacter` 0)) (== OtherActor (`self.Barril REF`)))
    (set `self.Presionando` false)
    (goto _label :!via `Reverse`)))

(fn `UserConstructionScript`)