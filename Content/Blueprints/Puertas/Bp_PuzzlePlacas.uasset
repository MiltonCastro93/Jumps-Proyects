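; Pressure-plate puzzle actor that opens a referenced door when three plates hold their target values, shown on text renders.
; Bp_Box actors tagged "Cubo" add their Value to a plate's running total on overlap.
; On exit, the total becomes the box's Value minus the total, rather than the reverse.
; Each change plays a sound and tests all three totals for exact matches before calling AbrirPuerta.
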(event `self.ReceiveBeginPlay`
  (`TextRenderComponent.K2_SetText` (`self.TextRenderA`) (`KismetTextLibrary.Conv_IntToText` (`self.ValorA`)))
  (`TextRenderComponent.K2_SetText` (`self.TextRenderB`) (`KismetTextLibrary.Conv_IntToText` (`self.ValorB`)))
  (`TextRenderComponent.K2_SetText` (`self.TextRenderC`) (`KismetTextLibrary.Conv_IntToText` (`self.ValorC`)))
  (`AudioComponent.Stop` (`self.Sound`)))

(event `self.Box1.OnComponentBeginOverlap`
  (params (OverlappedComponent :type "PrimitiveComponent Object Reference") (OtherActor :type "Actor Object Reference") (OtherComp :type "PrimitiveComponent Object Reference") (OtherBodyIndex :type Integer) (bFromSweep :type Boolean) (SweepResult :type "HitResult Structure (by ref)"))
  ;[0 0 0 0.5] Verifica si A esta OK
  (if (`self.ActorHasTag` OtherActor "Cubo")
    (bind _asbp_box (cast `/Game/Blueprints/Item/Bp_Box` OtherActor))
    (set `self.CurrentA` (+ (`/Game/Blueprints/Item/Bp_Box.Value` _asbp_box) (`self.CurrentA`)))
    (`self.EjecuteTest` :!label _label)))

(event `self.Box1.OnComponentEndOverlap`
  (params (OverlappedComponent :type "PrimitiveComponent Object Reference") (OtherActor :type "Actor Object Reference") (OtherComp :type "PrimitiveComponent Object Reference") (OtherBodyIndex :type Integer))
  ;[0 0 0 0.5] Verifica si A esta OK
  (if (`self.ActorHasTag` OtherActor "Cubo")
    (bind _asbp_box (cast `/Game/Blueprints/Item/Bp_Box` OtherActor))
    (set `self.CurrentA` (- (`/Game/Blueprints/Item/Bp_Box.Value` _asbp_box) (`self.CurrentA`)))
    (goto _label)))

(event `EjecuteTest`
  ;[0 0 0 0.5] Comprobacion Triple del puzzle para abrir
  (`AudioComponent.Play` (`self.Sound`) 0.0)
  (if (and (== (`self.ValorA`) (`self.CurrentA`)) (== (`self.ValorB`) (`self.CurrentB`)) (== (`self.ValorC`) (`self.CurrentC`)))
    (`/Game/Blueprints/Puertas/Bp_PuertaConPlaca.Abrir Puerta` (`self.PuertaREF`))))

(event `self.Box2.OnComponentBeginOverlap`
  (params (OverlappedComponent :type "PrimitiveComponent Object Reference") (OtherActor :type "Actor Object Reference") (OtherComp :type "PrimitiveComponent Object Reference") (OtherBodyIndex :type Integer) (bFromSweep :type Boolean) (SweepResult :type "HitResult Structure (by ref)"))
  ;[0 0 0 0.5] Verifica si la B esta OK
  (if (`self.ActorHasTag` OtherActor "Cubo")
    (bind _asbp_box (cast `/Game/Blueprints/Item/Bp_Box` OtherActor))
    (set `self.CurrentB` (+ (`/Game/Blueprints/Item/Bp_Box.Value` _asbp_box) (`self.CurrentB`)))
    (`self.EjecuteTest` :!label _label_2)))

(event `self.Box2.OnComponentEndOverlap`
  (params (OverlappedComponent :type "PrimitiveComponent Object Reference") (OtherActor :type "Actor Object Reference") (OtherComp :type "PrimitiveComponent Object Reference") (OtherBodyIndex :type Integer))
  ;[0 0 0 0.5] Verifica si la B esta OK
  (if (`self.ActorHasTag` OtherActor "Cubo")
    (bind _asbp_box (cast `/Game/Blueprints/Item/Bp_Box` OtherActor))
    (set `self.CurrentB` (- (`/Game/Blueprints/Item/Bp_Box.Value` _asbp_box) (`self.CurrentB`)))
    (goto _label_2)))

(event `self.Box3.OnComponentBeginOverlap`
  (params (OverlappedComponent :type "PrimitiveComponent Object Reference") (OtherActor :type "Actor Object Reference") (OtherComp :type "PrimitiveComponent Object Reference") (OtherBodyIndex :type Integer) (bFromSweep :type Boolean) (SweepResult :type "HitResult Structure (by ref)"))
  ;[0 0 0 0.5] Verifica si la C esta OK
  (if (`self.ActorHasTag` OtherActor "Cubo")
    (bind _asbp_box (cast `/Game/Blueprints/Item/Bp_Box` OtherActor))
    (set `self.CurrentC` (+ (`/Game/Blueprints/Item/Bp_Box.Value` _asbp_box) (`self.CurrentC`)))
    (`self.EjecuteTest` :!label _label_3)))

(event `self.Box3.OnComponentEndOverlap`
  (params (OverlappedComponent :type "PrimitiveComponent Object Reference") (OtherActor :type "Actor Object Reference") (OtherComp :type "PrimitiveComponent Object Reference") (OtherBodyIndex :type Integer))
  ;[0 0 0 0.5] Verifica si la C esta OK
  (if (`self.ActorHasTag` OtherActor "Cubo")
    (bind _asbp_box (cast `/Game/Blueprints/Item/Bp_Box` OtherActor))
    (set `self.CurrentC` (- (`/Game/Blueprints/Item/Bp_Box.Value` _asbp_box) (`self.CurrentC`)))
    (goto _label_3)))

(fn `UserConstructionScript`)